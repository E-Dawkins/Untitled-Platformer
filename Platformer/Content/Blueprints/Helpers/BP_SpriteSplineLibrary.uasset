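; Blueprint function library that lines a spline with Paper2D sprite components at fixed section-length intervals.
; SpawnSpritesAlongSpline adds one sprite component to the parent actor per full section, attaches it to the spline and sets its collision.
; Each is placed by distance along the spline and rotated to the tangent.
; A spawn type picks its sprite: uniform, random, start/end-capped, or array order forward or reversed.
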(fn `Get Random Sprite From Array`
  (params (`Sprite Array` :type "Array of PaperSprite Object Reference"))
  (returns (`Random Sprite` :type "PaperSprite Object Reference"))
  (return (`KismetArrayLibrary.Array_Random` `Sprite Array`)))

(fn `Get Sprite From Index`
  (params (Index :type Integer) (LastIndex :type Integer) (`Start Sprite` :type "PaperSprite Object Reference") (`End Sprite` :type "PaperSprite Object Reference") (`Middle Sprite` :type "PaperSprite Object Reference"))
  (returns (`Selected Sprite` :type "PaperSprite Object Reference"))
  (if (== Index 0)
    (return (`local.Start Sprite`))
    (elif (== (`local.Index`) (`local.LastIndex`))
      (return (`local.End Sprite`))
      (else
        (return (`local.Middle Sprite`))))))

(fn `Get Start Location / Rotation`
  (params (Index :type Integer) (SectionLength :type "Float (double-precision)") (Offset :type "Float (double-precision)") (Spline :type "SplineComponent Object Reference"))
  (returns (Position :type "Vector Structure") (Rotation :type "Rotator Structure"))
  (bind _returnvalue (+ Offset (* Index SectionLength)))
  (return (`SplineComponent.GetLocationAtDistanceAlongSpline` Spline _returnvalue "Local") (`KismetMathLibrary.Conv_VectorToRotator` (`KismetMathLibrary.ClampVectorSize` (`SplineComponent.GetTangentAtDistanceAlongSpline` Spline _returnvalue "Local") 0.0 SectionLength))))

(fn `Set Current Sprite`
  (params (SpriteSpawnType :type "/Game/Blueprints/Helpers/E_SpriteSplineSpawnType Enum" :default "NewEnumerator0") (Index :type Integer) (LastIndex :type Integer) (StartSprite :type "PaperSprite Object Reference") (EndSprite :type "PaperSprite Object Reference") (MiddleSprite :type "PaperSprite Object Reference") (RandomSprites :type "Array of PaperSprite Object Reference") (CurrentSpriteComponent :type "PaperSpriteComponent Object Reference"))
  (bind _returnvalue (- (`KismetArrayLibrary.Array_LastIndex` (`local.RandomSprites`)) (`local.Index`)))
  (switch `/Game/Blueprints/Helpers/E_SpriteSplineSpawnType` SpriteSpawnType
    (:`NewEnumerator0`
      ;[1 1 1] All same
      (`PaperSpriteComponent.SetSprite` (`local.CurrentSpriteComponent`) (`local.MiddleSprite`)))
    (:`NewEnumerator1`
      ;[1 1 1] All random
      (bind _random_sprite (`self.Get Random Sprite From Array` (`local.RandomSprites`)))
      (`PaperSpriteComponent.SetSprite` (`local.CurrentSpriteComponent`) _random_sprite))
    (:`NewEnumerator2`
      ;[1 1 1] Capped same
      (bind _selected_sprite (`self.Get Sprite From Index` (`local.Index`) (`local.LastIndex`) (`local.StartSprite`) (`local.EndSprite`) (`local.MiddleSprite`)))
      (`PaperSpriteComponent.SetSprite` (`local.CurrentSpriteComponent`) _selected_sprite))
    (:`NewEnumerator3`
      ;[1 1 1] Capped random
      (bind _random_sprite_2 (`self.Get Random Sprite From Array` (`local.RandomSprites`)))
      (bind _selected_sprite_2 (`self.Get Sprite From Index` (`local.Index`) (`local.LastIndex`) (`local.StartSprite`) (`local.EndSprite`) _random_sprite_2))
      (`PaperSpriteComponent.SetSprite` (`local.CurrentSpriteComponent`) _selected_sprite_2))
    (:`NewEnumerator4`
      ;[1 1 1] In order
      (if (`KismetArrayLibrary.Array_IsValidIndex` (`local.RandomSprites`) (`local.Index`))
        (`PaperSpriteComponent.SetSprite` (`local.CurrentSpriteComponent`) (`|GetArrayItem` (`local.RandomSprites`) (`local.Index`)))))
    (:`NewEnumerator5`
      (if (`KismetArrayLibrary.Array_IsValidIndex` (`local.RandomSprites`) _returnvalue)
        (`PaperSpriteComponent.SetSprite` (`local.CurrentSpriteComponent`) (`|GetArrayItem` (`local.RandomSprites`) _returnvalue))))))

(fn `Spawn Sprites Along Spline`
  (params (Spline :type "SplineComponent Object Reference") (CollisionType :type "ECollisionEnabled Enum" :default "NoCollision") (ParentActor :type "Actor Object Reference") (SpriteSpawnType :type "/Game/Blueprints/Helpers/E_SpriteSplineSpawnType Enum" :default "NewEnumerator0") (StartSprite :type "PaperSprite Object Reference") (EndSprite :type "PaperSprite Object Reference") (MiddleSprite :type "PaperSprite Object Reference") (RandomSprites :type "Array of PaperSprite Object Reference"))
  (locals (SectionLength :type "Float (double-precision)" :default 50.0) (Offset :type "Float (double-precision)" :default 25.0) (Index :type Integer) (LastIndex :type Integer) (`Current Sprite Component` :type "PaperSpriteComponent Object Reference"))
  ;[1 1 1] Loop over all full length sections of spline
  (bind _output_get (set `local.LastIndex` (- (`KismetMathLibrary.FTrunc` (`KismetMathLibrary.SafeDivide` (`SplineComponent.GetSplineLength` (`local.Spline`)) (`local.SectionLength`))) 1)))
  (for _index (range (+ _output_get 1))
    (set `local.Index` _index)
    ;[1 1 1] Create / attach sprite component, and set appropriate sprite
    (bind _returnvalue (`|AddComponentByClass` :`self` (`local.ParentActor`) :`Class` "/Script/Paper2D.PaperSpriteComponent" :`bManualAttachment` true))
    (bind _output_get_2 (set `local.Current Sprite Component` _returnvalue))
    (`SceneComponent.K2_AttachToComponent` _output_get_2 (`local.Spline`) "None" "KeepRelative" "KeepRelative" "KeepRelative" true)
    (`self.Set Current Sprite` (`local.SpriteSpawnType`) (`local.Index`) (`local.LastIndex`) (`local.StartSprite`) (`local.EndSprite`) (`local.MiddleSprite`) (`local.RandomSprites`) (`local.Current Sprite Component`))
    ;[1 1 1] Set default current sprite components' location, rotation and collision
    (bind (_position _rotation) (`self.Get Start Location / Rotation` (`local.Index`) (`local.SectionLength`) (`local.Offset`) (`local.Spline`)))
    (`SceneComponent.K2_SetRelativeLocationAndRotation` (`local.Current Sprite Component`) _position _rotation false false)
    (`PrimitiveComponent.SetCollisionEnabled` (`local.Current Sprite Component`) (`local.CollisionType`))))